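; Networked door actor for the KJMod VRP mod that players can open, lock, buy, sell, rename and share with co-owners.
; A timed local overlap check shows status UI and enables E/I interaction and the F2 management menu.
; Menu actions become named KJMod server events, with purchases and sales routed through a game-mode interface.
; RepNotifies refresh UI, play sounds and drive swing or move/rotate timeline animations.
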(event Custom|DetectOwningPlayerOverlap
  (bind _returnvalue (Game|GetPlayerController 0))
  ;[0 1 0.0959] BEGIN PLAY EVENT
  ;;[1 1 1] Is the local (me) pawn overlapping this doors collision zone? If so then show the UI
  (if (Collision|IsOverlappingActor (Variables|Default|GetCollisionBox) (Pawn|GetControlledPawn (Game|GetPlayerController 0)) :!class /Script/Engine.PrimitiveComponent)
    (if (and (not (Variables|UI|GetDoorUIVisible)) (not (Variables|UI|GetAdvancedDoorUIVisible)))
      ;;;[1 1 1] Add UI
      (Development|PrintString "Adding...")
      (Variables|UI|SetDoorUIVisible true)
      (Input|EnableInput _returnvalue)
      (bind _returnvalue_2 (UserInterface|CreateWidget "/Game/CustomContent/UGC2275057327/Doors/KJMod_VRP_DoorUIWidgetBP.KJMod_VRP_DoorUIWidgetBP_C" _returnvalue))
      (bind _output_get (Variables|UI|SetDoorUI _returnvalue_2))
      (UserInterface|Viewport|AddtoViewport _output_get 0)
      (CallFunction|ShowDoorStatus))
    (else
      (Utilities|FlowControl|Sequence
        (:then_0
          ;;;[1 1 1] Remove standard UI (seen my all)
          (if (Variables|UI|GetDoorUIVisible)
            (Development|PrintString "Removing..")
            (Variables|UI|SetDoorUIVisible false)
            (Widget|RemovefromParent (Variables|UI|GetDoorUI))
            (Variables|UI|SetDoorUI 0)
            (Input|DisableInput (Game|GetPlayerController 0))))
        (:then_1
          ;;;[1 1 1] Remove "Advanced" options (seen by door owner or server admin), remember this shows a mouse pointer so ensure we focus back on game
          (if (Variables|UI|GetAdvancedDoorUIVisible)
            (Variables|UI|SetAdvancedDoorUIVisible false)
            (Widget|RemovefromParent (Variables|UI|GetAdvancedDoorUI))
            (bind _returnvalue_3 (Class|KJModPlayerProxy|GetLocalPlayerProxyStatic))
            (Class|KJModPlayerProxy|SetInputMode _returnvalue_3 "GameFocused" (Variables|UI|GetAdvancedDoorUI)) ; Focus back on game
            (Variables|UI|SetAdvancedDoorUI 0)))))))

(event Custom|PlayLockedDoorSound
  ;[1 1 1] Interaction (server event)
  ;;[1 1 1] Let everyone hear the attempt
  (Audio|PlaySoundatLocation (Variables|Sounds|GetDoorLockedSoundCue) (Transformation|GetActorLocation) "0, 0, 0" 1.0 1.0 0.0 "/Game/CustomContent/UGC2275057327/Doors/Sounds/DoorSoundAttenuation.DoorSoundAttenuation" 0 0))

(event EventBeginPlay
  ;[0 1 0.0959] BEGIN PLAY EVENT
  (Utilities|HandleClientServerLogic
    (:ClientLogic
      (Utilities|Time|SetTimerbyEvent (delegate Custom|DetectOwningPlayerOverlap) 0.5 true) ; Test X times a second
    )))

(event EventPlayerInteracting
  (params (interactingPlayerProxy :type KJ%20Mod%20Player%20Proxy%20Object%20Reference) (playerController :type Player%20Controller%20Object%20Reference) (active :type Boolean) (inputChord :type Input%20Chord%20Structure) (cookie :type Integer))
  ;[1 1 1] Interaction (server event)
  (Utilities|GetInteractingKey inputChord
    (:E_Pressed
      (if true
        ;;[1 1 1] Not locked? open it
        (if (and (not (Variables|Locking|GetIsLocked)) (not (Variables|OpenClose|GetIsCycling)))
          (Variables|OpenClose|SetIsCycling true)
          (Variables|OpenClose|SetIsDoorOpen (not (Variables|OpenClose|GetIsDoorOpen)))
          (Utilities|FlowControl|Delay 1.0)
          (Variables|OpenClose|SetIsCycling false)
          (else
            (CallFunction|PlayLockedDoorSound)))))
    (:I_Pressed
      (if (Variables|Ownership|GetIsOwned)
        (bind _validowner (CallFunction|IsLocalPlayerOwnerorCoOwner interactingPlayerProxy))
        (if _validowner ; OWned by person pressing it?
          (Variables|Locking|SetIsLocked (not (Variables|Locking|GetIsLocked))))))))

(event EventReleaseOwnership
  ;[1 1 1] EVENT - Release Ownership - Occurs when GM releases (either forcably, or as a result of a sell)
  (Variables|Ownership|SetOwningSteamID "")
  (Variables|Ownership|SetOwningPlayerName "")
  (Variables|Ownership|SetIsOwned false) ; Owned by someone
)

(event EventSetDoorLocked
  (params (IsLocked :type Boolean))
  ;[1 1 1] Comment
  (bind _output_get (Variables|Locking|SetIsLocked IsLocked)))

(event EventSetDoorOwner
  (params (SteamID :type Integer) (PlayerName :type String))
  ;[1 1 1] We don't care about this, but must implement it to avoid a crash
)

(event Input|KeyboardEvents|F2
  (params (Key :type Key%20Structure :default "None"))
  ;[1 1 1] F2 Pressed (locally)
  (:Pressed
    (bind _returnvalue (Class|KJModPlayerProxy|GetLocalPlayerProxyStatic))
    (if (or (Utilities|Enum|Equal(Enum) (Variables|Ownership|GetOwningSteamID) (Utilities|GetInteractingProxySteamID _returnvalue)) (not (Variables|Ownership|GetIsOwned))) ; Not owned? or owned by me?
      (if (Variables|UI|GetAdvancedDoorUIVisible)
        (Widget|RemovefromParent (Variables|UI|GetAdvancedDoorUI))
        (bind _returnvalue_2 (Class|KJModPlayerProxy|GetLocalPlayerProxyStatic))
        (Class|KJModPlayerProxy|SetInputMode _returnvalue_2 "GameFocused" (Variables|UI|GetAdvancedDoorUI)) ; Remove mouse
        (Variables|UI|SetAdvancedDoorUI 0)
        (Variables|UI|SetAdvancedDoorUIVisible false)
        (else
          (bind _returnvalue_3 (UserInterface|CreateWidget "/Game/CustomContent/UGC2275057327/Doors/KJMod_VRP_DoorAdvancedUIWidgetBP.KJMod_VRP_DoorAdvancedUIWidgetBP_C" (Game|GetPlayerController 0) self))
          (bind _output_get (Variables|UI|SetAdvancedDoorUI _returnvalue_3))
          (UserInterface|Viewport|AddtoViewport _output_get 5)
          (bind _returnvalue_4 (Class|KJModPlayerProxy|GetLocalPlayerProxyStatic))
          (Class|KJModPlayerProxy|SetInputMode _returnvalue_4 "UserInterfaceFocused" _output_get) ; Show the mouse!
          (Variables|UI|SetAdvancedDoorUIVisible true)
          ;;[1 1 1] Remove normal UI
          (if (Variables|UI|GetDoorUIVisible)
            (Variables|UI|SetDoorUIVisible false)
            (Widget|RemovefromParent (Variables|UI|GetDoorUI))
            (Variables|UI|SetDoorUI 0)))))))

(event Input|KeyboardEvents|E
  (params (Key :type Key%20Structure :default "None"))
  ;[1 1 1] E Pressed (locally)
  (:Pressed
    (bind _returnvalue (Class|KJModPlayerProxy|GetLocalPlayerProxyStatic))
    (Class|KJModPlayerProxy|Interaction _returnvalue self false (Utilities|Struct|MakeInputChord Key false))))

(event Input|KeyboardEvents|I
  (params (Key :type Key%20Structure :default "None"))
  ;[1 1 1] I Pressed (locally)
  (:Pressed
    (bind _returnvalue (Class|KJModPlayerProxy|GetLocalPlayerProxyStatic))
    (Class|KJModPlayerProxy|Interaction _returnvalue self false (Utilities|Struct|MakeInputChord Key false))))

(event Custom|CloseDoorMulticast
  ;[1 1 1] Door open/close movement - must run on all clients (and server) to stay in sync
  (switch Utilities|FlowControl|Switch|SwitchonKJMod_VRP_OpenVisualisationEnum (Variables|SettingsVisualisation|GetVisualisationMode)
    (:NewEnumerator0
      (bind _doorangle (Timeline|Timeline_1 ReverseFromEnd)
        (:Update
          (Transformation|SetRelativeRotation (Variables|Default|GetHinge) (Math|Rotator|MakeRotator 0.0 0.0 (* _doorangle (Variables|SettingsVisualisation|GetMaxOpenAngle))) false false))))
    (:NewEnumerator1
      (bind _doorangle_2 (Timeline|Timeline_3 ReverseFromEnd)
        (:Update
          (Transformation|SetRelativeLocationAndRotation (Variables|Default|GetHinge) (Math|Vector|Lerp(Vector) "0, 0, 0" (Variables|SettingsVisualisation|GetMoveToRelativeOffset) _doorangle_2) (Math|Rotator|Lerp(Rotator) "0, 0, 0" (Variables|SettingsVisualisation|GetRotateToRelative) _doorangle_2 true) false true))))))

(event Custom|OpenDoorMulticast
  ;[1 1 1] Door open/close movement - must run on all clients (and server) to stay in sync
  (switch Utilities|FlowControl|Switch|SwitchonKJMod_VRP_OpenVisualisationEnum (Variables|SettingsVisualisation|GetVisualisationMode)
    (:NewEnumerator0
      (bind _doorangle (Timeline|Timeline_0 PlayFromStart)
        (:Update
          (Transformation|SetRelativeRotation (Variables|Default|GetHinge) (Math|Rotator|MakeRotator 0.0 0.0 (* _doorangle (Variables|SettingsVisualisation|GetMaxOpenAngle))) false false))))
    (:NewEnumerator1
      (bind _doorangle_2 (Timeline|Timeline_2 PlayFromStart)
        (:Update
          (Transformation|SetRelativeLocationAndRotation (Variables|Default|GetHinge) (Math|Vector|Lerp(Vector) "0, 0, 0" (Variables|SettingsVisualisation|GetMoveToRelativeOffset) _doorangle_2) (Math|Rotator|Lerp(Rotator) "0, 0, 0" (Variables|SettingsVisualisation|GetRotateToRelative) _doorangle_2 true) false true))))))

(event Custom|UI_CloseAdvanced
  ;[1 1 1] CLOSE UI
  (Widget|RemovefromParent (Variables|UI|GetAdvancedDoorUI))
  (bind _returnvalue (Class|KJModPlayerProxy|GetLocalPlayerProxyStatic))
  (Class|KJModPlayerProxy|SetInputMode _returnvalue "GameFocused" (Variables|UI|GetAdvancedDoorUI)) ; Remove mouse
  (Variables|UI|SetAdvancedDoorUI 0)
  (Variables|UI|SetAdvancedDoorUIVisible false))

(event Custom|UI_BuyDoor
  ;[1 1 1] UI - Buy Door
  (CallFunction|UICloseAdvanced)
  (bind _returnvalue (Class|KJModActorEvents|CreateEvent "BuyDoor"))
  (Class|KJModActorEvents|ExecuteEvent self (Game|GetPlayerController 0) _returnvalue))

(event Custom|UI_ChangeTitle
  (params (DoorTitle :type String))
  ;[1 1 1] UI  - Change Title; construct a KJMod event and send it to "us" (on the server!") - received in "KJMod Events" EventGraph
  (bind _returnvalue (Class|KJModActorEvents|CreateEvent "ChangeTitle"))
  (Class|KJModActorEvents|AddStringParameter _returnvalue "Name" DoorTitle)
  (Class|KJModActorEvents|ExecuteEvent self (Game|GetPlayerController 0) _returnvalue))

(event Custom|UI_SetOwnership
  (params (Disallow :type Boolean))
  ;[1 1 1] Disallow Ownership
  (CallFunction|UICloseAdvanced)
  (bind _returnvalue (Class|KJModActorEvents|CreateEvent "SetOwnership"))
  (Class|KJModActorEvents|AddBoolParameter _returnvalue "Disallow" Disallow)
  (Class|KJModActorEvents|ExecuteEvent self (Game|GetPlayerController 0) _returnvalue))

(event Custom|UI_ModifyCoowner
  (params (Add :type Boolean) (SteamID :type String) (PlayerName :type String))
  ;[1 1 1] Modify Coowner
  (bind _returnvalue (Class|KJModActorEvents|CreateEvent (Utilities|String|SelectString "AddCoowner" "RemoveCoowner" Add)))
  (Class|KJModActorEvents|AddStringParameter _returnvalue "SteamID" SteamID)
  (Class|KJModActorEvents|AddStringParameter _returnvalue "Playername" PlayerName)
  (Class|KJModActorEvents|ExecuteEvent self (Game|GetPlayerController 0) _returnvalue))

(event Custom|UI_SellDoor
  ;[1 1 1] UI - Sell Door
  (CallFunction|UICloseAdvanced)
  (bind _returnvalue (Class|KJModActorEvents|CreateEvent "SellDoor"))
  (Class|KJModActorEvents|ExecuteEvent self (Game|GetPlayerController 0) _returnvalue))

(event Custom|SetOwnershipEvent
  (params (ActorEvent :type KJ%20Mod%20Actor%20Events%20Object%20Reference))
  (bind _returnvalue (Class|KJModActorEvents|GetCalleePlayerController ActorEvent))
  (bind _uniquenetid (Class|AdvancedSessionsLibrary|GetUniqueNetID _returnvalue))
  (bind _string (Class|AdvancedSessionsLibrary|UniqueNetIdtoString _uniquenetid))
  ;[1 1 1] Change Title Event
  (bind _returnvalue_2 (Class|KJModUtilityActor|IsAdminPlayer 0 _string))
  (if _returnvalue_2
    (Variables|Ownership|SetDoorCanBeOwned (not (Class|KJModActorEvents|GetBoolField ActorEvent "Disallow")))
    (CallFunction|SellDoorEvent ActorEvent)
    (else
      (Class|KJModProxy|PrintStringKJMod 0 (Utilities|String|Append "Player (" (Class|AdvancedSessionsLibrary|GetPlayerName _returnvalue) " - " _string ")" " Is not admin, but tried to disallow door ownership") true true "(R=0.000000,G=1.000000,B=0.000000,A=1.000000)" 5.0))))

(event Custom|SellDoorEvent
  (params (Target :type KJ%20Mod%20Actor%20Events%20Object%20Reference))
  ;[1 1 1] Sell Door Event
  (bind _interface (Utilities|GetGameModeDoorInterface)
    (:Out
      (Default|NotificationOfSale _interface self)
      (CallFunction|ReleaseOwnership))))

(event Custom|ChangeTitleEvent
  (params (ActorEvent :type KJ%20Mod%20Actor%20Events%20Object%20Reference))
  ;[1 1 1] Change Title Event
  (Variables|Settings|SetDisplayName (Class|KJModActorEvents|GetStringParam ActorEvent "Name")))

(event Custom|BuyDoorEvent
  (params (Target :type KJ%20Mod%20Actor%20Events%20Object%20Reference))
  ;[1 1 1] Buy Door Event
  (if (Variables|Ownership|GetDoorCanBeOwned)
    (bind _returnvalue (Class|KJModPlayerProxy|GetPlayerProxy 0 (Class|KJModActorEvents|GetCalleePlayerController Target)))
    (bind _interface (Utilities|GetGameModeDoorInterface)
      (:Out
        (bind (_granted _steamid _playername) (Default|RequesttoOwn _interface _returnvalue self (Variables|Settings|GetMetaData))) ; Ask GM can we own it
        (if _granted
          (Variables|Ownership|SetOwningSteamID _steamid)
          (Variables|Ownership|SetOwningPlayerName _playername)
          (Variables|Ownership|SetIsOwned true) ; Owned by someone
        )))))

(event Custom|RemoveCoOwnerEvent
  (params (Target :type KJ%20Mod%20Actor%20Events%20Object%20Reference))
  ;[1 1 1] Add or remove coowner
  (bind _index (CallFunction|FindCoOwner (Class|KJModActorEvents|GetStringParam Target "SteamID")))
  (if (>= _index 0)
    (Utilities|Array|RemoveIndex (Variables|Ownership|GetCo_Owners) _index)))

(event Custom|AddCoOwnerEvent
  (params (Target :type KJ%20Mod%20Actor%20Events%20Object%20Reference))
  (bind _returnvalue (Class|KJModActorEvents|GetStringParam Target "SteamID"))
  ;[1 1 1] Add or remove coowner
  (bind _index (CallFunction|FindCoOwner _returnvalue))
  (if (< _index 0)
    (Utilities|Array|Add (Variables|Ownership|GetCo_Owners) (Utilities|Struct|MakeKJMod_VRP_OwnerInfo (Class|KJModActorEvents|GetStringParam Target "Playername") _returnvalue))))

(event EventServerActorEvent
  (params (actorEvent :type KJ%20Mod%20Actor%20Events%20Object%20Reference))
  ;[1 1 1] SERVER - ACTOR EVENT - all KJMod events are received here
  (switch string (Class|KJModActorEvents|GetEventName actorEvent)
    (:ChangeTitle
      (CallFunction|ChangeTitleEvent actorEvent))
    (:BuyDoor
      (CallFunction|BuyDoorEvent actorEvent))
    (:SellDoor
      (CallFunction|SellDoorEvent actorEvent))
    (:SetOwnership
      (CallFunction|SetOwnershipEvent actorEvent))
    (:AddCoowner
      (CallFunction|AddCoOwnerEvent actorEvent))
    (:RemoveCoowner
      (CallFunction|RemoveCoOwnerEvent actorEvent))))

(fn ConstructionScript)

(fn OnRepIsDoorOpen
  (if (Variables|OpenClose|GetIsDoorOpen)
    (CallFunction|OpenDoorMulticast)
    (Audio|PlaySoundatLocation (Variables|Sounds|GetOpenDoorSoundCue) (Transformation|GetActorLocation) "0, 0, 0" 1.0 1.0 0.0 "/Game/CustomContent/UGC2275057327/Doors/Sounds/DoorSoundAttenuation.DoorSoundAttenuation" 0 0)
    (else
      (CallFunction|CloseDoorMulticast)
      (Audio|PlaySoundatLocation (Variables|Sounds|GetCloseDoorSoundCue) (Transformation|GetActorLocation) "0, 0, 0" 1.0 1.0 0.0 "/Game/CustomContent/UGC2275057327/Doors/Sounds/DoorSoundAttenuation.DoorSoundAttenuation" 0 0))))

(fn ShowDoorStatus
  (if (Variables|UI|GetDoorUIVisible)
    (Utilities|IsValid (Variables|UI|GetDoorUI) ; We can be asked when the player is not at the door..
      (:Is%20Valid
        ;[1 1 1] We can be the "owner" but also "co-owner"
        (bind _returnvalue (Class|KJModPlayerProxy|GetLocalPlayerProxyStatic))
        (bind _validowner (CallFunction|IsLocalPlayerOwnerorCoOwner _returnvalue))
        (Default|ShowStatus (Variables|UI|GetDoorUI) (Variables|Ownership|GetIsOwned) (Variables|Ownership|GetIsOwnedByUs) _validowner (Variables|Locking|GetIsLocked) (Variables|OpenClose|GetIsDoorOpen) (Variables|Settings|GetDisplayName) (Variables|Ownership|GetOwningPlayerName) (Variables|Settings|GetOwnershipPrice) (Variables|Ownership|GetDoorCanBeOwned))))))

(fn CallBackEvent
  (params (SomeValue :type String))
  (Development|PrintString SomeValue))

(fn OnRepIsOwned
  ;[1 1 1] Ownership changed, show (if we can)
  (CallFunction|ShowDoorStatus))

(fn OnRepOwningSteamID
  (Variables|Ownership|SetIsOwnedByUs (Utilities|Enum|Equal(Enum) (Variables|Ownership|GetOwningSteamID) (Class|AdvancedSessionsLibrary|UniqueNetIdtoString (Class|AdvancedSessionsLibrary|GetUniqueNetIDfromPlayerState (Variables|/Script/Engine.Controller|GetPlayerState (Game|GetPlayerController 0))))))
  (CallFunction|ShowDoorStatus))

(fn ClearDoorStatus
  (bind _doorui (Variables|UI|GetDoorUI))
  (if (Variables|UI|GetDoorUIVisible)
    (Utilities|IsValid _doorui ; e can be asked when the player is not at the door..
      (:Is%20Valid
        (Default|ClearStatus _doorui)))))

(fn OnRepIsLocked
  ;[1 1 1] Lock status changed..
  (CallFunction|ShowDoorStatus)
  (if (Variables|Locking|GetIsLocked)
    (Audio|PlaySoundatLocation (Variables|Sounds|GetLockDoorSoundCue) (Transformation|GetActorLocation) "0, 0, 0" 1.0 1.0 0.0 "/Game/CustomContent/UGC2275057327/Doors/Sounds/DoorSoundAttenuation.DoorSoundAttenuation" 0 0)))

(fn FindCoOwner
  (params (SteamID :type String))
  (for (_array_element _array_index) (Variables|Ownership|GetCo_Owners)
    (if (Utilities|Enum|Equal(Enum) (Utilities|Struct|BreakKJMod_VRP_OwnerInfo _array_element) SteamID)
      (return _array_index)))
  (return -1))

(fn IsLocalPlayerOwnerorCoOwner
  (params (PlayerProxy :type KJ%20Mod%20Player%20Proxy%20Object%20Reference))
  (bind _steamid (Utilities|GetInteractingProxySteamID PlayerProxy))
  (if (Utilities|Enum|Equal(Enum) (Variables|Ownership|GetOwningSteamID) _steamid) ; Is normal owner us?
    (return true)
    (else
      (for _array_element (Variables|Ownership|GetCo_Owners)
        (if (Utilities|Enum|Equal(Enum) (.CoOwner_SteamID (Utilities|Struct|BreakKJMod_VRP_OwnerInfo _array_element)) _steamid) ; Is this a coowner?
          (return true)))
      (return false))))

(fn GetInfo
  (return (Variables|Settings|GetDisplayName) (Variables|Settings|GetOwnershipPrice) ""))